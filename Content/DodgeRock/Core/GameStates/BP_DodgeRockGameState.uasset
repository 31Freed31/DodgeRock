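; Game state for DodgeRock that runs the round timer, scoring and end-of-round flow.
; A looping one-second timer counts time played, adds the current rock count to the player's score and passes elapsed time to the game mode's Process.
; EndGame stops the timer, submits the score to the game instance as highest score, then asks the game mode to restart after a short delay.
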(event `self.ReceiveBeginPlay`
  (`|ExecutionSequence`
    (:`then_0`
      (bind _asbp_dodge_rock_game_mode (cast `/Game/DodgeRock/Core/GameModes/BP_DodgeRockGameMode` (`GameplayStatics.GetGameMode`)))
      (set `self.DodgeModeGameRock` _asbp_dodge_rock_game_mode))
    (:`then_1`
      (bind _asbp_dodge_rock_player_state (cast `/Game/DodgeRock/Core/PlayerStates/BP_DodgeRockPLayerState` (`GameplayStatics.GetPlayerState` 0)))
      (set `self.DodgeRockPlayerState` _asbp_dodge_rock_player_state)
      (`self.StartGame`))))

(event `StartGame`
  (bind _returnvalue (`KismetSystemLibrary.K2_SetTimerDelegate` (`|CreateDelegate` :!event `CoregameTimeEvent`) 1.0 true))
  (set `self.CoreGameTimer` _returnvalue)
  (set `self.IsGameEnded` false))

(event `EndGame`
  (`KismetSystemLibrary.K2_ClearAndInvalidateTimerHandle` (`self.CoreGameTimer`))
  (set `self.IsGameEnded` true)
  (`|ExecutionSequence`
    (:`then_0`
      (bind _asbp_dodge_rock_game_instance (cast `/Game/DodgeRock/Core/GameInstance/BP_DodgeRockGameInstance` (`GameplayStatics.GetGameInstance`)))
      (bind _dodgerockplayerstate (`self.DodgeRockPlayerState`)
        (:`then`
          (`/Game/DodgeRock/Core/GameInstance/BP_DodgeRockGameInstance.SetHighestScore` _asbp_dodge_rock_game_instance (`/Game/DodgeRock/Core/PlayerStates/BP_DodgeRockPLayerState.GetPlayerScore` _dodgerockplayerstate)))
        (:`else`)))
    (:`then_1`
      (`KismetSystemLibrary.Delay` 3.0)
      (bind _dodgemodegamerock (`self.DodgeModeGameRock`)
        (:`then`
          (`/Game/DodgeRock/Core/GameModes/BP_DodgeRockGameMode.RestartGame` _dodgemodegamerock))
        (:`else`)))))

(event `RestartGame`
  (bind _returnvalue (`GameplayStatics.GetCurrentLevelName` true))
  (`GameplayStatics.OpenLevel` (`KismetStringLibrary.Conv_StringToName` _returnvalue)))

(event `CoregameTimeEvent`
  (`/Engine/EditorBlueprintResources/StandardMacros.IncrementInt` (`self.TimePlayed`)
    (:`  `
      (`|ExecutionSequence`
        (:`then_0`
          (bind _dodgerockplayerstate (`self.DodgeRockPlayerState`)
            (:`then`
              (`/Game/DodgeRock/Core/PlayerStates/BP_DodgeRockPLayerState.SetPlayerScore` _dodgerockplayerstate (+ (`/Game/DodgeRock/Core/PlayerStates/BP_DodgeRockPLayerState.GetPlayerScore` _dodgerockplayerstate) (`self.GetRockCount`))))
            (:`else`)))
        (:`then_1`
          (bind _dodgemodegamerock (`self.DodgeModeGameRock`)
            (:`then`
              (`/Game/DodgeRock/Core/GameModes/BP_DodgeRockGameMode.Process` _dodgemodegamerock (`self.TimePlayed`)))
            (:`else`)))))))

(fn `GetRockCount`
  (returns (RockCount :type Integer))
  (return (`self.RockCount`)))

(fn `SetRockCount`
  (params (RockCount :type Integer))
  (set `self.RockCount` RockCount))

(fn `UserConstructionScript`)