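; BP_DodgeRockHUD is the HUD for DodgeRock, switching between the player interface and the death screen.
; On BeginPlay it creates and shows WBP_PlayerInterface, then binds to the OnOwnerDied event of the owning BP_DodgeRockCharacter's health component.
; The death handler, OnPlyerDied, removes the player interface and adds WBP_DeathScreen to the viewport.
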(event `self.ReceiveBeginPlay`
  (bind _returnvalue (`|CreateWidget` "/Game/DodgeRock/UI/WBP_PlayerInterface.WBP_PlayerInterface_C" (`GameplayStatics.GetPlayerController` 0)))
  (bind _output_get (set `self.PlayerInterfaceWidget` _returnvalue))
  (`UserWidget.AddToViewport` _output_get 0)
  (bind _asbp_dodge_rock_character (cast `/Game/DodgeRock/Characters/BP_DodgeRockCharacter` (`self.GetOwningPawn`)))
  (add `/Game/DodgeRock/Blueprints/ActorComponents/BP_HealthComponent.OnOwnerDied` (`/Game/DodgeRock/Characters/BP_DodgeRockCharacter.BP_HealthComponent` _asbp_dodge_rock_character) (`|CreateDelegate` :!event `OnPlyerDied`)))

(event `OnPlyerDied`
  (`|ExecutionSequence`
    (:`then_0`
      (bind _playerinterfacewidget (`self.PlayerInterfaceWidget`)
        (:`then`
          (`Widget.RemoveFromParent` _playerinterfacewidget))
        (:`else`)))
    (:`then_1`
      (bind _returnvalue (`|CreateWidget` "/Game/DodgeRock/UI/WBP_DeathScreen.WBP_DeathScreen_C" (`GameplayStatics.GetPlayerController` 0)))
      (set `self.DeathScreenWidget` _returnvalue)
      (`UserWidget.AddToViewport` _returnvalue 0))))

(fn `UserConstructionScript`)